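; PlayerCamera is a player-controlled pawn in the ProceduralCity project that flies or moves along the view direction and picks points in the world.
; Axis inputs drive movement and controller pitch and yaw.
; Left click runs a debug-drawn Visibility line trace from the camera, appending hit points to RaycastOutputPoint and saving the new index.
; Undo removes the entry at that saved index without updating the index afterwards.
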(event EventBeginPlay)

(event Input|ActionEvents|InputActionLeftClick
  (params (Key :type Key%20Structure :default "None"))
  (bind _playercamera (Variables|Default|GetPlayerCamera))
  (bind _returnvalue (Transformation|GetWorldLocation _playercamera))
  ;[1 1 1] ShotRaycast
  (:Pressed
    (bind (_outhit _returnvalue_2) (Collision|LineTraceByChannel _returnvalue (+ _returnvalue (* (Math|Vector|GetForwardVector (Transformation|GetWorldRotation _playercamera)) 1.5e+03)) "TraceTypeQuery1" false 0 "ForDuration"))
    ;[1 1 1] Store RaycastOutput
    (if _returnvalue_2
      (bind _returnvalue_3 (Utilities|Array|Add (Variables|Default|GetRaycastOutputPoint) (.impactpoint _outhit)))
      (Variables|Default|SetRaycastIndex _returnvalue_3))))

(event Input|ActionEvents|InputActionUndo
  (params (Key :type Key%20Structure :default "None"))
  (:Pressed
    (Utilities|Array|RemoveIndex (Variables|Default|GetRaycastOutputPoint) (Variables|Default|GetRaycastIndex))))

(event Input|AxisEvents|InputAxisMoveForward
  (params (AxisValue :type Float%20%28single-precision%29))
  ;[1 1 1] PawnMovement
  (Pawn|Input|AddMovementInput (Math|Vector|GetForwardVector (Pawn|GetControlRotation :!class /Script/Engine.Pawn)) AxisValue false))

(event Input|AxisEvents|InputAxisMoveLeft
  (params (AxisValue :type Float%20%28single-precision%29))
  ;[1 1 1] PawnMovement
  (Pawn|Input|AddMovementInput (Math|Vector|GetRightVector (Pawn|GetControlRotation :!class /Script/Engine.Pawn)) AxisValue false))

(event Input|AxisEvents|InputAxisLookVertical
  (params (AxisValue :type Float%20%28single-precision%29))
  ;[1 1 1] PawnRotation
  (Pawn|Input|AddControllerPitchInput AxisValue))

(event Input|AxisEvents|InputAxisLookHorizontal
  (params (AxisValue :type Float%20%28single-precision%29))
  ;[1 1 1] PawnRotation
  (Pawn|Input|AddControllerYawInput AxisValue))

(fn ConstructionScript)