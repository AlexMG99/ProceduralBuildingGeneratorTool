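; Player pawn in the ProceduralCity folder with axis-driven movement, mouse look and a debug raycast on left click.
; Movement input follows the control rotation's forward and right vectors, while look axes feed controller pitch and yaw.
; Left click traces the Visibility channel 1500 units forward from the movement component's updated primitive, drawing persistent debug lines without using the hit result.
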(event Input|ActionEvents|InputActionLeftClick
  (params (Key :type Key%20Structure :default "None"))
  (bind _charactermovement (Variables|Character|GetCharacterMovement))
  (bind _updatedprimitive (Variables|/Script/Engine.MovementComponent|GetUpdatedPrimitive _charactermovement))
  (bind _returnvalue (Transformation|GetWorldLocation _updatedprimitive))
  ;[1 1 1] ShotRaycast
  (:Pressed
    (Collision|LineTraceByChannel _returnvalue (+ _returnvalue (* (Math|Vector|GetForwardVector (Transformation|GetWorldRotation (Variables|/Script/Engine.MovementComponent|GetUpdatedPrimitive _charactermovement))) 1.5e+03)) "TraceTypeQuery1" false 0 "Persistent")))

(event Input|AxisEvents|InputAxisMoveForward
  (params (AxisValue :type Float%20%28single-precision%29))
  ;[1 1 1] PawnMovement
  (Pawn|Input|AddMovementInput (Math|Vector|GetForwardVector (Pawn|GetControlRotation :!class /Script/Engine.Pawn)) AxisValue false))

(event Input|AxisEvents|InputAxisMoveLeft
  (params (AxisValue :type Float%20%28single-precision%29))
  ;[1 1 1] PawnMovement
  (Pawn|Input|AddMovementInput (Math|Vector|GetRightVector (Pawn|GetControlRotation :!class /Script/Engine.Pawn)) AxisValue false))

(event Input|AxisEvents|InputAxisLookVertical
  (params (AxisValue :type Float%20%28single-precision%29))
  (Pawn|Input|AddControllerPitchInput AxisValue))

(event Input|AxisEvents|InputAxisLookHorizontal
  (params (AxisValue :type Float%20%28single-precision%29))
  (Pawn|Input|AddControllerYawInput AxisValue))

(fn ConstructionScript)